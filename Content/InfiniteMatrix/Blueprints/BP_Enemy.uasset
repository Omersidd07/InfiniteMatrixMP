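; BP_Enemy is a short-lived hazard actor that damages the player on contact.
; Overlap on its Enemy component casts to BP_Player, directly subtracts a fixed amount from Health, then plays a world camera shake, a 2D sound and a debug message.
; A timer started on BeginPlay destroys the actor after a few seconds; hitting the player does not destroy it.
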(event `self.ReceiveBeginPlay`
  (`KismetSystemLibrary.K2_SetTimer` null "DestroyEnemy" 4.0))

(event `self.ReceiveTick`
  (params (DeltaSeconds :type "Float (single-precision)")))

(event `self.Enemy.OnComponentBeginOverlap`
  (params (OverlappedComponent :type "PrimitiveComponent Object Reference") (OtherActor :type "Actor Object Reference") (OtherComp :type "PrimitiveComponent Object Reference") (OtherBodyIndex :type Integer) (bFromSweep :type Boolean) (SweepResult :type "HitResult Structure (by ref)"))
  (bind _asbp_player (cast `/Game/InfiniteMatrix/Blueprints/BP_Player` OtherActor))
  (set `/Game/InfiniteMatrix/Blueprints/BP_Player.Health` (- (`/Game/InfiniteMatrix/Blueprints/BP_Player.Health` _asbp_player) 10.0) _asbp_player)
  (`GameplayStatics.PlayWorldCameraShake` "/Game/InfiniteMatrix/Blueprints/daShake.daShake_C" (`self.K2_GetActorLocation`) 0.0 500.0)
  (`GameplayStatics.PlaySound2D` "/Game/bruhCollision.bruhCollision" 1.0 1.0 0.0 null null)
  (`KismetSystemLibrary.PrintString` "OUCH!" true true (struct :`R` 0.244792 :`G` 0.022715 :`B` 0.032458 :`A` 1.0)))

(fn `DestroyEnemy`
  (`self.K2_DestroyActor`))

(fn `UserConstructionScript`)