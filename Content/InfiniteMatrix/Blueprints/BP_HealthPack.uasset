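; BP_HealthPack is a short-lived health pickup for the player.
; On BeginPlay it starts a timer that destroys it after a few seconds if it is not collected.
; When BP_Player overlaps the HealthPack component below full health, it adds a fixed amount of health without clamping, plays a sound and destroys itself.
; At full health it only prints a debug message and stays in place.
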(event `self.ReceiveBeginPlay`
  (`KismetSystemLibrary.K2_SetTimer` null "DestroyHealthPack" 4.0))

(event `self.ReceiveTick`
  (params (DeltaSeconds :type "Float (single-precision)")))

(event `self.HealthPack.OnComponentBeginOverlap`
  (params (OverlappedComponent :type "PrimitiveComponent Object Reference") (OtherActor :type "Actor Object Reference") (OtherComp :type "PrimitiveComponent Object Reference") (OtherBodyIndex :type Integer) (bFromSweep :type Boolean) (SweepResult :type "HitResult Structure (by ref)"))
  (bind _asbp_player (cast `/Game/InfiniteMatrix/Blueprints/BP_Player` OtherActor))
  (if (>= (`/Game/InfiniteMatrix/Blueprints/BP_Player.Health` _asbp_player) 100.0)
    (`KismetSystemLibrary.PrintString` "HEALTH ALREADY FULL" true true (struct :`R` 1.0 :`G` 0.04144 :`B` 0.802577 :`A` 1.0))
    (else
      (`KismetSystemLibrary.PrintString` "HEALTH INCREASED" true true (struct :`R` 1.0 :`G` 0.039631 :`B` 0.830314 :`A` 1.0))
      (set `/Game/InfiniteMatrix/Blueprints/BP_Player.Health` (+ (`/Game/InfiniteMatrix/Blueprints/BP_Player.Health` _asbp_player) 10.0) _asbp_player)
      (`GameplayStatics.PlaySound2D` "/Game/noiceee.noiceee" 1.0 1.0 0.0 null null)
      (`self.K2_DestroyActor`))))

(fn `DestroyHealthPack`
  (`self.K2_DestroyActor`))

(fn `UserConstructionScript`)